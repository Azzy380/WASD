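; WASD mod Blueprint that adds camera-relative keyboard movement to a game with a SetDestination click input.
; Tick force-feeds the WASD vector to character movement when montage checks allow, turns control rotation to match, and ignores normal move input.
; Forced input bypasses that ignore, which SetDestination resets once WASD is idle.
; Space snaps actor and control rotation toward the held direction for a directed dash.
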(event `self.ReceiveTick`
  (params (DeltaSeconds :type "Float (single-precision)"))
  (bind _returnvalue (`GameplayStatics.GetPlayerController` 0))
  (bind _returnvalue_2 (`self.get WSAD input`))
  (bind _returnvalue_3 (`SkeletalMeshComponent.GetAnimInstance` (`Character.Mesh` (`GameplayStatics.GetPlayerCharacter` 0))))
  (bind _returnvalue_4 (`AnimInstance.IsAnyMontagePlaying` _returnvalue_3))
  (bind _returnvalue_5 (`AnimInstance.GetCurrentActiveMontage` _returnvalue_3))
  ;[1 1 1] WSAD
  (if (and (`self.Is WASD Input`) (or (not _returnvalue_4) (and _returnvalue_4 (and (== (`AnimInstance.Montage_GetCurrentSection` _returnvalue_3 _returnvalue_5) "Default") (== (`AnimInstance.Montage_GetPlayRate` _returnvalue_3 _returnvalue_5) 1.0) (`KismetStringLibrary.StartsWith` (`KismetSystemLibrary.GetDisplayName` _returnvalue_3) "AnimMontage")))))
    (`PawnMovementComponent.AddInputVector` (`Character.CharacterMovement` (`GameplayStatics.GetPlayerCharacter` 0)) _returnvalue_2 true)
    (`Controller.SetControlRotation` _returnvalue (`KismetMathLibrary.Conv_VectorToRotator` _returnvalue_2))
    (`Controller.SetIgnoreMoveInput` _returnvalue true)))

(event `InputAction|SetDestination` :consume false
  (params (Key :type "Key Structure"))
  ;[1 1 1] WSAD
  (:`Pressed`
    (if (not (`self.Is WASD Input`)) :!label _label
      (`Controller.ResetIgnoreMoveInput` (`GameplayStatics.GetPlayerController` 0))))
  (:`Released`
    (goto _label)))

(event `Key|SpaceBar` :consume false
  (params (Key :type "Key Structure"))
  (bind _returnvalue (`GameplayStatics.GetPlayerCharacter` 0))
  (bind _returnvalue_2 (`KismetMathLibrary.Conv_VectorToRotator` (+ (* (`self.get WSAD input`) 100.0) (`KismetMathLibrary.Conv_RotatorToVector` (`self.K2_GetActorRotation` _returnvalue)))))
  ;[1 1 1] directed dash
  (:`Pressed`
    (if (> (`KismetMathLibrary.VSize` (`KismetMathLibrary.Vector_GetAbs` (`self.get WSAD input`))) 0.1)
      (`self.K2_SetActorRotation` _returnvalue _returnvalue_2 false)
      (`Controller.SetControlRotation` (`Pawn.GetController` _returnvalue) _returnvalue_2))))

(fn `NewFunction_0`)

(fn `UserConstructionScript`)